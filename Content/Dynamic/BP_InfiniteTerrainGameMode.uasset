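; Game mode for an endless tiled terrain that builds the starting run of tiles and tracks the score.
; On BeginPlay it fills a pool of nav mesh bounds volumes, then spawns tiles in a loop up to MaxTiles.
; Each spawned BP_Tile receives the shared volume pool and supplies the attach transform where the next tile spawns.
; NewTileConquered increments the score.
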(event EventBeginPlay
  (Class|TGInfiniteTerrainGameMode|PopulateBoundsVolumePool)
  (for _index (range 0 (Variables|Default|GetMaxTiles))
    (CallFunction|SpawnTile)))

(fn ConstructionScript)

(fn SpawnTile
  (bind _returnvalue (Game|SpawnActorfromClass "/Game/Dynamic/Terrain/Props/BP_Tile.BP_Tile_C" (Variables|Default|GetnextTileTransform) "Undefined" 0 0))
  (Class|TGTile|SetPool _returnvalue (Variables|Default|GetNavMeshBoundsVolumePool))
  (bind _attach_transform (Default|GetAttachLocation _returnvalue))
  (Variables|Default|SetnextTileTransform _attach_transform))

(fn NewTileConquered
  (Math|Integer|IncrementInt (Variables|Default|GetScore)))